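; Enemy character Blueprint that loads speed and damage from DT_Enemies, by chosen type or random row, with optional overrides.
; AI perception puts a living player into the blackboard as target; Attack damages pawns via forward line trace.
; Death or capsule overlap triggers physics ragdoll, disabling sight and clearing the target, while Tick moves the actor to the pelvis.
; Bodies are destroyed after a delay; heavy damage only schedules an empty StandUp event.
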(event `self.ReceiveBeginPlay`
  (bind _ac_health (`self.AC_Health`))
  (add `/Game/UnrealJam2025/Components/AC_Health.OnDeath` _ac_health (`|CreateDelegate` :!event `OnDeath`))
  (add `/Game/UnrealJam2025/Components/AC_Health.OnHealthUpdated` _ac_health (`|CreateDelegate` :!event `OnHealthUpdated`))
  (set `self.InitialMeshTransform` (`SceneComponent.GetRelativeTransform` (`self.Mesh`)))
  (if (`self.OverrideType`)
    (bind _returnvalue (`|GetDataTableRow` "/Game/UnrealJam2025/Data/DT_Enemies.DT_Enemies" (`KismetStringLibrary.Conv_StringToName` (`|GetEnumeratorNameAsString` (`self.Type`))))
      (:`then`
        (`self.SetDataTablesValue` _returnvalue)))
    (else
      (bind _outrownames (`DataTableFunctionLibrary.GetDataTableRowNames` "/Game/UnrealJam2025/Data/DT_Enemies.DT_Enemies"))
      (bind _returnvalue_2 (`|GetDataTableRow` "/Game/UnrealJam2025/Data/DT_Enemies.DT_Enemies" (`|GetArrayItem` _outrownames (`KismetMathLibrary.RandomInteger` (`KismetArrayLibrary.Array_Length` _outrownames))))
        (:`then`
          (`self.SetDataTablesValue` _returnvalue_2))))))

(event `OnDeath`
  (`self.StartRagdolling` true)
  (`KismetSystemLibrary.K2_SetTimerDelegate` (delegate `Destroy`) (`self.TimeBeforeDestroyBody`)))

(event `Destroy`
  (bind _returnvalue_location (`KismetMathLibrary.BreakTransform` (`SkinnedMeshComponent.GetBoneTransform` (`self.Mesh`) "pelvis" "RTS_Actor")))
  (`AddComponent|NODE_AddNiagaraComponent-0` :`RelativeTransform` (`KismetMathLibrary.MakeTransform` _returnvalue_location))
  ; Find a way to keep particle alive even if actor is destroyed
  (`KismetSystemLibrary.Delay` 0.5)
  (`self.K2_DestroyActor`))

(event `self.AIPerception.OnTargetPerceptionUpdated`
  (params (Actor :type "Actor Object Reference") (Stimulus :type "AIStimulus Structure"))
  ; only check player
  (cast `/Game/UnrealJam2025/Blueprints/BP_Player` Actor)
  (bind _healthcomponent (message `/Game/UnrealJam2025/Interfaces/BPI_Damagable.GetHealthComponent` Actor))
  (`/Engine/EditorBlueprintResources/StandardMacros.IsValid` _healthcomponent
    (:`Is Valid`
      (add `/Game/UnrealJam2025/Components/AC_Health.OnDeath` _healthcomponent (delegate `OnTargetDeath`))
      (if (not (`/Game/UnrealJam2025/Components/AC_Health.IsDead` _healthcomponent))
        (`BlackboardComponent.SetValueAsObject` (`AIBlueprintHelperLibrary.GetBlackboard` null) "TargetActor" Actor)))))

(event `OnTargetDeath`
  (`self.ClearTarget`))

(event `Attack`
  (bind _capsulecomponent (`self.CapsuleComponent`))
  (bind _returnvalue (`SceneComponent.K2_GetComponentLocation` _capsulecomponent))
  (bind (_outhit _returnvalue_2) (`KismetSystemLibrary.LineTraceSingleForObjects` _returnvalue (+ _returnvalue (* (`SceneComponent.GetForwardVector` _capsulecomponent) (`self.AttackDistance`))) (`|MakeArray` "ObjectTypeQuery3" :!type "EObjectTypeQuery Enum")))
  (if _returnvalue_2
    (bind (_bblockinghit _binitialoverlap _time _distance _location _impactpoint _normal _impactnormal _physmat _hitactor) (`GameplayStatics.BreakHitResult` _outhit))
    (`GameplayStatics.ApplyPointDamage` _hitactor (`self.AttackDamage`) _normal _outhit (`self.GetController` self) self "/Script/Engine.DamageType")))

(event `OnHealthUpdated`
  (params (HealthDelta :type "Float (double-precision)"))
  (if (<= HealthDelta (- 0.0 (`self.DamageToFallThreshold`)))
    (`KismetSystemLibrary.K2_SetTimerDelegate` (delegate `StandUp`) (`self.TimeBeforeStandingUp`))))

(event `StandUp`)

(event `WakeUp`
  (`self.StopRagdolling`))

(event `self.CapsuleComponent.OnComponentBeginOverlap`
  (params (OverlappedComponent :type "PrimitiveComponent Object Reference") (OtherActor :type "Actor Object Reference") (OtherComp :type "PrimitiveComponent Object Reference") (OtherBodyIndex :type Integer) (bFromSweep :type Boolean) (SweepResult :type "HitResult Structure (by ref)"))
  (`self.StartRagdolling` false)
  (`PrimitiveComponent.SetSimulatePhysics` (`self.CapsuleComponent`) true))

(event `self.ReceiveTick`
  (params (DeltaSeconds :type "Float (single-precision)"))
  (if (`self.IsRagdolling`)
    (`self.RagdollUpdate`)))

(fn `ClearTarget`
  (`BlackboardComponent.SetValueAsObject` (`AIBlueprintHelperLibrary.GetBlackboard` null) "TargetActor" null))

(fn `GetHealthComponent`
  (returns (HealthComponent :type "/Game/UnrealJam2025/Components/AC_Health Object Reference"))
  (return (`self.AC_Health`)))

(fn `RagdollUpdate`
  (locals (RagdollFaceUp :type Boolean) (TargetRagdollRotation :type "Rotator Structure") (TargetRagdollLocation :type "Vector Structure"))
  (bind _yaw (.yaw (`SceneComponent.GetSocketRotation` (`self.Mesh`) "pelvis")))
  (`|ExecutionSequence`
    (:`then_0`
      ; Update target values
      (set `local.TargetRagdollLocation` (`SceneComponent.GetSocketLocation` (`self.Mesh`) "pelvis"))
      (bind _output_get (set `local.RagdollFaceUp` (< (.roll (`SceneComponent.GetSocketRotation` (`self.Mesh`) "pelvis")) 0.0)))
      (set `local.TargetRagdollRotation` (`KismetMathLibrary.MakeRotator` 0.0 0.0 (select `bool` _output_get :`false` _yaw :`true` (- _yaw 180.0) :!type "Float (double-precision)"))))
    (:`then_1`
      (`self.K2_SetActorLocationAndRotation` (`local.TargetRagdollLocation`) (`local.TargetRagdollRotation`)))))

(fn `SetDataTablesValue`
  (params (Row :type "/Game/UnrealJam2025/Structs/S_Enemy Structure"))
  (bind (_type _speed _damage) (break `/Game/UnrealJam2025/Structs/S_Enemy` Row))
  (`|ExecutionSequence`
    (:`then_0`
      (if (not (`self.OverrideSpeed`))
        (bind _output_get (set `self.WalkSpeed` _speed))
        (set `CharacterMovementComponent.MaxWalkSpeed` _output_get (`self.CharacterMovement`))))
    (:`then_1`
      (if (not (`self.OverrideDamage`))
        (set `self.AttackDamage` _damage)))))

(fn `StartRagdolling`
  (params (DisableCapsuleCollision :type Boolean))
  (bind _mesh (`self.Mesh`))
  (`|ExecutionSequence`
    (:`then_0`
      (`CharacterMovementComponent.SetMovementMode` (`self.CharacterMovement`) "MOVE_None" 0)
      (`AIPerceptionComponent.SetSenseEnabled` (`self.AIPerception`) "/Script/AIModule.AISense_Sight" false)
      (`self.ClearTarget`)
      (`NavMovementInterface.StopActiveMovement` (`self.CharacterMovement`))
      (`PrimitiveComponent.SetCollisionProfileName` _mesh "Ragdoll" true)
      (`SkeletalMeshComponent.SetAllBodiesBelowSimulatePhysics` _mesh "root" true true)
      (set `self.IsRagdolling` true))
    (:`then_1`
      (if DisableCapsuleCollision
        (`PrimitiveComponent.SetCollisionEnabled` (`self.CapsuleComponent`) "NoCollision")))))

(fn `StopRagdolling`
  (bind _mesh (`self.Mesh`))
  (`AIPerceptionComponent.SetSenseEnabled` (`self.AIPerception`) "/Script/AIModule.AISense_Sight" true)
  (`PrimitiveComponent.SetCollisionProfileName` _mesh "CharacterMesh" true)
  (`SkeletalMeshComponent.SetAllBodiesSimulatePhysics` _mesh false)
  (`SceneComponent.K2_SetRelativeTransform` _mesh (`self.InitialMeshTransform`) false false)
  (`PrimitiveComponent.SetCollisionEnabled` (`self.CapsuleComponent`) "QueryAndPhysics")
  (set `self.IsRagdolling` false))

(fn `UserConstructionScript`)