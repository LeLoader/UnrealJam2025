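; BP_Lever is an interactable lever that drops objects into a spawning zone.
; Interact calls Activate, which flips the State flag and runs DropObjects when the flag was off.
; DropObjects spawns one actor for each ObjectTypes entry at a random point inside the referenced SpawningZone's box.
; Switching back off only prints a reset message and leaves spawned objects untouched.
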(event `/Game/UnrealJam2025/Interfaces/BPI_Interactable.Interact`
  (params (Instigator :type "Actor Object Reference") (Component :type "SceneComponent Object Reference"))
  (`self.Activate`))

(fn `Activate`
  (if (`self.State`)
    (`KismetSystemLibrary.PrintString` "Reset state")
    (else
      (`self.DropObjects`)))
  (set `self.State` (not (`self.State`))))

(fn `DropObjects`
  (bind _box (`/Game/UnrealJam2025/Blueprints/BP_SpawningZone.Box` (`self.SpawningZone`)))
  (for _array_element (`self.ObjectTypes`)
    (`|SpawnActorFromClass` _array_element (`KismetMathLibrary.MakeTransform` (`KismetMathLibrary.RandomPointInBoundingBox` (`SceneComponent.K2_GetComponentLocation` _box) (`BoxComponent.GetScaledBoxExtent` _box))) "Undefined" "MultiplyWithRoot" null null)))

(fn `UserConstructionScript`)