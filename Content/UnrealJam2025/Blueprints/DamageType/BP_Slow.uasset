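; BP_Slow is a damage-type effect meant to temporarily slow a target's walk speed.
; Unconnected nodes in ApplyEffect would scale the target's MaxWalkSpeed by SlowAmount and set a timer by name for DeapplyEffect after Duration.
; Unconnected nodes in DeapplyEffect would divide MaxWalkSpeed by SlowAmount to undo it.
; Both function entries are unwired, so the effect currently does nothing.
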(fn `ApplyEffect`
  (params (Target :type "Character Object Reference")))

(fn `DeapplyEffect`)