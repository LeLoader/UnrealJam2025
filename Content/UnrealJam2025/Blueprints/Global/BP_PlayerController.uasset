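; BP_PlayerController is the player controller Blueprint that opens the pause menu when the IA_Pause input action starts.
; If the IsPauseMenuOpen flag is unset, it sets it, then creates and displays WBP_PauseMenu.
; It then switches to UI-only input focused on the widget, shows the mouse cursor and pauses the game.
; This graph only opens the menu and never clears the flag.
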(event `EnhancedInput|/Game/UnrealJam2025/Inputs/Actions/IA_Pause`
  (params (ActionValue :type Boolean) (ElapsedSeconds :type "Float (double-precision)") (TriggeredSeconds :type "Float (double-precision)") (InputAction :type "InputAction Object Reference" :default "/Game/UnrealJam2025/Inputs/Actions/IA_Pause.IA_Pause"))
  (bind _returnvalue (`GameplayStatics.GetPlayerController` 0))
  (:`Started`
    (if (not (`self.bIsPauseMenuOpen`))
      (set `self.bIsPauseMenuOpen` true)
      (bind _returnvalue_2 (`|CreateWidget` "/Game/UnrealJam2025/Widgets/WBP_PauseMenu.WBP_PauseMenu_C" _returnvalue))
      (bind _output_get (set `self.PauseMenuWidget` _returnvalue_2))
      (`UserWidget.AddToViewport` _output_get 0)
      (`WidgetBlueprintLibrary.SetInputMode_UIOnlyEx` _returnvalue (`self.PauseMenuWidget`) "DoNotLock" true)
      (set `PlayerController.bShowMouseCursor` true (`GameplayStatics.GetPlayerController` 0))
      (`GameplayStatics.SetGamePaused` true))))

(fn `UserConstructionScript`)