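; Game mode that sets up the starting UI and steps the game through narrated acts.
; BeginPlay adds the main and subtitle widgets, switches to UI-only input with a cursor, and caches the level's BP_Lever.
; NextAct increments the act index and calls OnActStart, which hands that act's data table to the lever and shows CurrentAct's intro text through BP_PlayerController.
; OnActEnd is an empty stub.
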(event `self.ReceiveBeginPlay`
  (bind _returnvalue (`GameplayStatics.GetPlayerController` 0))
  (bind _returnvalue_2 (`|CreateWidget` "/Game/UnrealJam2025/Widgets/WBP_Widget.WBP_Widget_C" _returnvalue))
  (`UserWidget.AddToViewport` _returnvalue_2 0)
  (`WidgetBlueprintLibrary.SetInputMode_UIOnlyEx` _returnvalue null "DoNotLock" true)
  (set `PlayerController.bShowMouseCursor` true _returnvalue)
  (bind _returnvalue_3 (`GameplayStatics.GetActorOfClass` "/Game/UnrealJam2025/Blueprints/BP_Lever.BP_Lever_C"))
  (set `self.Lever` _returnvalue_3)
  (bind _returnvalue_4 (`|CreateWidget` "/Game/UnrealJam2025/Widgets/WBP_Subtitle.WBP_Subtitle_C" (`GameplayStatics.GetPlayerController` 0)))
  (`UserWidget.AddToViewport` _returnvalue_4 0)
  (set `self.SubtitleWidgetRef` _returnvalue_4))

(event `OnActStart`
  (bind _output (`|GetArrayItem` (`self.DataTables`) (`self.CurrentActIndex`)))
  (bind _introtext (`/Game/UnrealJam2025/Blueprints/BP_ActNarration.IntroText` (`self.CurrentAct`)))
  (`/Engine/EditorBlueprintResources/StandardMacros.IsValid` _output
    (:`Is Valid`
      (set `/Game/UnrealJam2025/Blueprints/BP_Lever.CurrentDataTable` _output (`self.Lever`))
      (`/Engine/EditorBlueprintResources/StandardMacros.IsValid` (`|GetArrayItem` (`self.DataAssets`) (`self.CurrentActIndex`))
        (:`Is Valid`
          (bind _asbp_player_controller (cast `/Game/UnrealJam2025/Blueprints/Global/BP_PlayerController` (`GameplayStatics.GetPlayerController` 0)))
          (`/Game/UnrealJam2025/Blueprints/Global/BP_PlayerController.ShowNarration` _asbp_player_controller _introtext 2.0)
          (`KismetSystemLibrary.PrintText` _introtext))))))

(event `OnActEnd`)

(event `NextAct`
  (if (not (== (`KismetArrayLibrary.Array_Length` (`self.DataTables`)) 0))
    (set `self.CurrentActIndex` (+ (`self.CurrentActIndex`) 1))
    (`self.OnActStart`)))

(fn `UserConstructionScript`)