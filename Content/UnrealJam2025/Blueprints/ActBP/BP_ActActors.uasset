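; BP_ActActors is a container of child actors, including pickups, that moves along a spline during an act transition.
; BeginPlay gathers FakeRoot's children, disables pickup physics and collision, and snaps to the start of BP_ActObjectsTransition's spline.
; StartTransition runs a duration-scaled timeline that moves every component to the same point along the first spline segment, then fires OnTransitionEnded.
; Helpers to respawn children as standalone actors and restore collision exist but are not called here.
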(event `self.ReceiveBeginPlay`
  (set `self.Root` (`self.FakeRoot`))
  (`self.AttachEverything`)
  (`self.DisableCollision`)
  (bind _returnvalue (`GameplayStatics.GetActorOfClass` "/Game/UnrealJam2025/Blueprints/ActBP/BP_ActObjectsTransition.BP_ActObjectsTransition_C"))
  (bind _output_get (set `self.Spline` (`/Game/UnrealJam2025/Blueprints/ActBP/BP_ActObjectsTransition.Spline` _returnvalue)))
  (`self.K2_SetActorLocation` (`SplineComponent.GetLocationAtSplineInputKey` _output_get 0.0 "World")))

(event `StartTransition`
  (bind _spline (`self.Spline`))
  (`TimelineComponent.SetPlayRate` (`self.Transition`) (/ 1.0 (`self.TransitionDuration`)))
  (bind (_direction _alpha) (`Timeline|Transition`)
    (:`Update`
      (bind _returnvalue (`SplineComponent.GetLocationAtDistanceAlongSpline` _spline (`KismetMathLibrary.Lerp` 0.0 (`SplineComponent.GetDistanceAlongSplineAtSplineInputKey` _spline 1.0) _alpha) "World"))
      (`KismetSystemLibrary.PrintString` (`KismetStringLibrary.Conv_VectorToString` _returnvalue))
      (for _array_element (`self.AllComps`)
        (`SceneComponent.K2_SetWorldLocation` _array_element _returnvalue false false)))
    (:`Finished`
      (`self.OnTransitionEnded`))))

(fn `AttachEverything`
  (for _index (range (`SceneComponent.GetNumChildrenComponents` (`self.Root`)))
    (bind _returnvalue (`SceneComponent.GetChildComponent` (`self.Root`) _index))
    (`SceneComponent.K2_AttachToComponent` _returnvalue (`self.FakeRoot`) "None" "KeepWorld" "KeepWorld" "KeepWorld" true)
    (`KismetArrayLibrary.Array_Add` (`self.AllComps`) _returnvalue)))

(fn `DetachEverything`
  (for _array_element (`self.AllComps`)
    (bind _aschild_actor_component (cast `ChildActorComponent` _array_element))
    (bind _asbp_pickup (cast `/Game/UnrealJam2025/Blueprints/BP_Pickup` (`ChildActorComponent.ChildActor` _aschild_actor_component))
      (:`then`
        (bind _returnvalue (`SceneComponent.K2_GetComponentToWorld` _aschild_actor_component))
        (`|SpawnActorFromClass` "/Game/UnrealJam2025/Blueprints/BP_Pickup.BP_Pickup_C" _returnvalue "Undefined" "MultiplyWithRoot" null (`/Game/UnrealJam2025/Blueprints/BP_Pickup.Definition` _asbp_pickup) null))
      (:`CastFailed`
        (`|SpawnActorFromClass` (`ChildActorComponent.ChildActorClass` _aschild_actor_component) _returnvalue "Undefined" "MultiplyWithRoot" null null)))))

(fn `DisableCollision`
  (for _array_element (`self.AllComps`)
    (bind _aschild_actor_component (cast `ChildActorComponent` _array_element))
    (bind _asbp_pickup (cast `/Game/UnrealJam2025/Blueprints/BP_Pickup` (`ChildActorComponent.ChildActor` _aschild_actor_component)))
    (bind _sm_pickup (`/Game/UnrealJam2025/Blueprints/BP_Pickup.SM_Pickup` _asbp_pickup))
    (`PrimitiveComponent.SetSimulatePhysics` _sm_pickup false)
    (`PrimitiveComponent.SetCollisionEnabled` _sm_pickup "NoCollision")))

(fn `ReactivateCollision`
  (for _array_element (`self.AllComps`)
    (bind _aschild_actor_component (cast `ChildActorComponent` _array_element))
    (bind _asbp_pickup (cast `/Game/UnrealJam2025/Blueprints/BP_Pickup` (`ChildActorComponent.ChildActor` _aschild_actor_component)))
    (bind _sm_pickup (`/Game/UnrealJam2025/Blueprints/BP_Pickup.SM_Pickup` _asbp_pickup))
    (`PrimitiveComponent.SetCollisionEnabled` _sm_pickup "QueryAndPhysics")
    (`PrimitiveComponent.SetSimulatePhysics` _sm_pickup true)))

(fn `UserConstructionScript`)