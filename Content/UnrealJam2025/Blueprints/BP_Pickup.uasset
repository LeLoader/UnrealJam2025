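; Data-driven physics pickup that the player can carry and throw to damage actors.
; A Definition supplies mesh, mass, sounds and damage; Interact attaches it with physics off, and Throw detaches it, applies an impulse and arms damage.
; Hits deal point or radial damage to new BPI_Damagable targets, destroying the pickup at its use limit.
; Tick disarms throw damage once it slows, using a next-frame gate to skip the initial zero velocity.
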(event `self.ReceiveBeginPlay`
  (`self.Init Object`))

(event `Init Object`
  (bind _sm_pickup (`self.SM_Pickup`))
  (`PrimitiveComponent.SetMassOverrideInKg` _sm_pickup "None" (`/Game/UnrealJam2025/Blueprints/BP_Object.Mass` (`self.Definition`)) true)
  (`StaticMeshComponent.SetStaticMesh` _sm_pickup (`/Game/UnrealJam2025/Blueprints/BP_Object.StaticMesh` (`self.Definition`))))

(event `self.SM_Pickup.OnComponentHit`
  (params (HitComponent :type "PrimitiveComponent Object Reference") (OtherActor :type "Actor Object Reference") (OtherComp :type "PrimitiveComponent Object Reference") (NormalImpulse :type "Vector Structure") (Hit :type "HitResult Structure (by ref)"))
  (bind _definition (`self.Definition`))
  (bind _definition_2 (`self.Definition`))
  (bind _currentusecount (`self.CurrentUseCount`))
  (if (and (`self.WillDamage`) (`KismetSystemLibrary.DoesImplementInterface` OtherActor "/Game/UnrealJam2025/Interfaces/BPI_Damagable.BPI_Damagable_C"))
    (bind _returnvalue (`KismetArrayLibrary.Array_AddUnique` (`self.AlreadyHitTargets`) OtherActor))
    (if (not (== _returnvalue -1))
      (if (`/Game/UnrealJam2025/Blueprints/BP_Object.IsExplosive` (`self.Definition`))
        (`GameplayStatics.ApplyRadialDamage` :`BaseDamage` (`/Game/UnrealJam2025/Blueprints/BP_Object.Damage` _definition) :`Origin` (`self.K2_GetActorLocation`) :`DamageRadius` (`/Game/UnrealJam2025/Blueprints/BP_Object.ExplosionRaidus` _definition) :`DamageTypeClass` (`/Game/UnrealJam2025/Blueprints/BP_Object.DamageType` _definition) :`DamageCauser` null :`InstigatedByController` null :`bDoFullDamage` true :`DamagePreventionChannel` "ECC_Vehicle")
        (else
          (`GameplayStatics.ApplyPointDamage` OtherActor (`/Game/UnrealJam2025/Blueprints/BP_Object.Damage` _definition_2) NormalImpulse Hit (`GameplayStatics.GetPlayerController` 0) self (`/Game/UnrealJam2025/Blueprints/BP_Object.DamageType` _definition_2))))
      (`GameplayStatics.SpawnSoundAttached` (`/Game/UnrealJam2025/Blueprints/BP_Object.ImpactSound` (`self.Definition`)) HitComponent "None" (`.Location` (`GameplayStatics.BreakHitResult` Hit)) (struct) "KeepRelativeOffset" false 1.0 1.0 0.0 null null)
      (bind _result (`/Engine/EditorBlueprintResources/StandardMacros.IncrementInt` _currentusecount)
        (:`  `
          (`|ExecutionSequence`
            (:`then_0`
              (if (>= _result (`/Game/UnrealJam2025/Blueprints/BP_Object.MaxUseBeforeDestroy` (`self.Definition`)))
                (`self.K2_DestroyActor`)))
            (:`then_1`
              (if (== _currentusecount 0)
                _))))))))

(event `TimeDilation`
  ; dilatation
  (`GameplayStatics.SetGlobalTimeDilation` 1.0))

(event `self.ReceiveTick`
  (params (DeltaSeconds :type "Float (single-precision)"))
  (if (`self.CanDamage`)
    (`KismetSystemLibrary.K2_SetTimerForNextTickDelegate` (delegate `Open`))
    (`/Engine/EditorBlueprintResources/StandardMacros.Gate` true :!label _label
      (:`Exit`
        (if (< (`KismetMathLibrary.VSize` (`SceneComponent.GetComponentVelocity` (`self.SM_Pickup`))) 10.0)
          (set `self.CanDamage` false)
          (goto _label :!via `Close`))))))

(event `Open`
  (goto _label :!via `Open`))

(event `/Game/UnrealJam2025/Interfaces/BPI_Interactable.Interact`
  (params (Instigator :type "Actor Object Reference") (Component :type "SceneComponent Object Reference"))
  (`self.Pickup` Component))

(fn `Pickup`
  (params (AttachComp :type "SceneComponent Object Reference"))
  (`self.SetPhysics` false)
  (`self.K2_AttachToComponent` AttachComp "None" "SnapToTarget" "SnapToTarget" "KeepWorld" false)
  (`KismetArrayLibrary.Array_Clear` (`self.AlreadyHitTargets`))
  (`GameplayStatics.PlaySound2D` (`/Game/UnrealJam2025/Blueprints/BP_Object.PickupSound` (`self.Definition`)) 1.0 1.0 0.0 null null)
  (return))

(fn `SetPhysics`
  (params (Activated :type Boolean))
  (if Activated
    (`PrimitiveComponent.SetSimulatePhysics` (`self.SM_Pickup`) true)
    (`PrimitiveComponent.SetEnableGravity` (`self.SM_Pickup`) true)
    (`PrimitiveComponent.SetCollisionEnabled` (`self.SM_Pickup`) "QueryAndPhysics")
    (else
      (`PrimitiveComponent.SetSimulatePhysics` (`self.SM_Pickup`) false)
      (`PrimitiveComponent.SetEnableGravity` (`self.SM_Pickup`) false)
      (`PrimitiveComponent.SetCollisionEnabled` (`self.SM_Pickup`) "NoCollision"))))

(fn `Throw`
  (params (Impulse :type "Vector Structure"))
  (bind _sm_pickup (`self.SM_Pickup`))
  (`self.K2_DetachFromActor` "KeepWorld" "KeepWorld" "KeepWorld")
  (`self.SetPhysics` true)
  (`PrimitiveComponent.AddImpulse` _sm_pickup Impulse "None" true)
  (`GameplayStatics.SpawnSoundAttached` (`/Game/UnrealJam2025/Blueprints/BP_Object.ThrowSound` (`self.Definition`)) _sm_pickup "None" (0.0 0.0 0.0) (struct) "KeepRelativeOffset" false 1.0 1.0 0.0 null null)
  (set `self.CanDamage` true)
  (return))

(fn `UserConstructionScript`)

(fn `WillDamage`
  (returns (WillDamage :type Boolean))
  (return (or (`self.CanDamage`) (`self.CanDamageWithoutThrow`))))