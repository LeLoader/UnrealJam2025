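; BP_NextActZone is a trigger zone, apparently marking the move to the next act, that detects the player and controls a spotlight.
; On BeginPlay it binds the sphere overlap, caches the light's intensity and plays a light sound at its location.
; An overlap by BP_Player fires the PlayerInZone dispatcher.
; SwitchLight turns the spotlight on or off by restoring the cached intensity or setting it to zero.
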(event `self.ReceiveBeginPlay`
  (add `PrimitiveComponent.OnComponentBeginOverlap` (`self.Sphere`) (delegate `OnComponentBeginOverlap`))
  (set `self.Intensity` (`LightComponentBase.Intensity` (`Light.LightComponent` (`self.Light`))))
  (`GameplayStatics.PlaySoundAtLocation` (`self.LightSound`) (`self.K2_GetActorLocation`) (struct) 1.0 1.0 0.0 null null null null))

(event `OnComponentBeginOverlap`
  (params (OverlappedComponent :type "PrimitiveComponent Object Reference") (OtherActor :type "Actor Object Reference") (OtherComp :type "PrimitiveComponent Object Reference") (OtherBodyIndex :type Integer) (bFromSweep :type Boolean) (SweepResult :type "HitResult Structure (by ref)"))
  (cast `/Game/UnrealJam2025/Blueprints/BP_Player` OtherActor)
  (`self.PlayerInZone`))

(fn `SwitchLight`
  (params (Active :type Boolean))
  (bind _spotlightcomponent (`SpotLight.SpotLightComponent` (`self.Light`)))
  (if Active
    (`LightComponent.SetIntensity` _spotlightcomponent (`self.Intensity`))
    (else
      (`LightComponent.SetIntensity` _spotlightcomponent 0.0))))

(fn `UserConstructionScript`)