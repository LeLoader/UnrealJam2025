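; Actor component that tracks health and death for its owner.
; On BeginPlay it fills health to max and binds to the owner's OnTakeAnyDamage, routing damage into ReceiveDamage.
; Damage and healing go through SetHealth with clamping, which broadcasts the health delta and triggers Death at or below a tolerance threshold.
; Death sets IsDead to block further changes, unbinds damage and fires OnDeath.
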(event `self.ReceiveBeginPlay`
  (`self.SetHealth` (`self.MaxHealth`))
  (add `Actor.OnTakeAnyDamage` (`self.GetOwner`) (delegate `OnTakeAnyDamage`)))

(event `OnTakeAnyDamage`
  (params (DamagedActor :type "Actor Object Reference") (Damage :type "Float (single-precision)") (DamageType :type "DamageType Object Reference") (InstigatedBy :type "Controller Object Reference") (DamageCauser :type "Actor Object Reference"))
  (`self.ReceiveDamage` Damage))

(event `Death`
  (set `self.IsDead` true)
  (remove `Actor.OnTakeAnyDamage` (`self.GetOwner`) (delegate `OnTakeAnyDamage`))
  (`self.OnDeath`)
  (`KismetSystemLibrary.PrintString` "Entity died"))

(fn `ReceiveDamage`
  (params (DamageAmount :type "Float (double-precision)"))
  (`self.SetHealth` (`KismetMathLibrary.FMax` (- (`self.CurrentHealth`) DamageAmount))))

(fn `ReceiveHeal`
  (params (HealAmount :type "Float (double-precision)"))
  (`self.SetHealth` (`KismetMathLibrary.FMin` (+ HealAmount (`self.CurrentHealth`)) (`self.MaxHealth`))))

(fn `SetHealth`
  (params (NewHealth :type "Float (double-precision)"))
  (locals (OldCurrentHealth :type "Float (double-precision)"))
  (set `local.OldCurrentHealth` (`self.CurrentHealth`))
  (if (not (`self.IsDead`))
    (bind _output_get (set `self.CurrentHealth` NewHealth))
    (`self.OnHealthUpdated` (- (`self.CurrentHealth`) (`local.OldCurrentHealth`)))
    (`KismetSystemLibrary.PrintString` (`KismetStringLibrary.Concat_StrStr` "New HP: " (`KismetStringLibrary.Conv_DoubleToString` _output_get)))
    (if (<= (`self.CurrentHealth`) (`self.DeathHealthTolerance`))
      (`self.Death`))))